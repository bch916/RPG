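; Spawner actor that places an overworld enemy (Slime, Warg, Magus or Goot, chosen by EnemyType) at its own transform.
; Shortly after BeginPlay it spawns immediately if IsActive, otherwise waits and makes a single random roll of ChanceToSpawn against ChanceConstant.
; SpawnEnemy stores the enemy, sets its MySpawner back-reference and clears IsActive.
; ActivateSpawner only sets the flag again, without spawning.
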(event `self.ReceiveBeginPlay`
  (`KismetSystemLibrary.Delay` 0.2)
  (if (`self.isActive`)
    (`self.spawnEnemy`)
    (else
      (`KismetSystemLibrary.Delay` 5.0)
      (bind _shouldspawn (`self.rollChanceToSpawn`))
      (if _shouldspawn
        (`self.spawnEnemy`)))))

(event `self.ReceiveTick`
  (params (DeltaSeconds :type "Float (single-precision)")))

(fn `activateSpawner`
  (set `self.isActive` true))

(fn `rollChanceToSpawn`
  (returns (shouldSpawn :type Boolean))
  (return (<= (`KismetMathLibrary.RandomFloatInRange` 0.0 (`self.chanceConstant`)) (`self.chanceToSpawn`))))

(fn `spawnEnemy`
  (switch `/Game/BlueprintsAndMaps/Blueprints/EnemyBPs/EnemyTypeEnum` (`self.enemyType`)
    (:`NewEnumerator0`
      (bind _returnvalue (`|SpawnActorFromClass` "/Game/BlueprintsAndMaps/Blueprints/EnemyBPs/Demo_BPs/overWorldEnemyPawnBP.overWorldEnemyPawnBP_C" (`self.GetTransform`) "Undefined" "OverrideRootScale" null 0 null))
      (bind _output_get (set `self.spawnedEnemy` _returnvalue))
      (set `/Game/BlueprintsAndMaps/Blueprints/EnemyBPs/Demo_BPs/overWorldEnemyPawnBP.mySpawner` self _output_get))
    (:`NewEnumerator1`
      (bind _returnvalue_2 (`|SpawnActorFromClass` "/Game/BlueprintsAndMaps/Blueprints/EnemyBPs/Demo_BPs/warg_enemyBP.warg_enemyBP_C" (`self.GetTransform`) "Undefined" "OverrideRootScale" null 0 null))
      (bind _output_get_2 (set `self.spawnedEnemy` _returnvalue_2))
      (set `/Game/BlueprintsAndMaps/Blueprints/EnemyBPs/Demo_BPs/overWorldEnemyPawnBP.mySpawner` self _output_get_2))
    (:`NewEnumerator2`
      (bind _returnvalue_3 (`|SpawnActorFromClass` "/Game/BlueprintsAndMaps/Blueprints/EnemyBPs/Demo_BPs/magus_enemyBP.magus_enemyBP_C" (`self.GetTransform`) "Undefined" "OverrideRootScale" null 0 null))
      (bind _output_get_3 (set `self.spawnedEnemy` _returnvalue_3))
      (set `/Game/BlueprintsAndMaps/Blueprints/EnemyBPs/Demo_BPs/overWorldEnemyPawnBP.mySpawner` self _output_get_3))
    (:`NewEnumerator3`
      (bind _returnvalue_4 (`|SpawnActorFromClass` "/Game/BlueprintsAndMaps/Blueprints/EnemyBPs/Demo_BPs/goot_enemyBP.goot_enemyBP_C" (`self.GetTransform`) "Undefined" "OverrideRootScale" null 0 null))
      (bind _output_get_4 (set `self.spawnedEnemy` _returnvalue_4))
      (set `/Game/BlueprintsAndMaps/Blueprints/EnemyBPs/Demo_BPs/overWorldEnemyPawnBP.mySpawner` self _output_get_4)))
  (set `self.isActive` false)
  (return))

(fn `UserConstructionScript`)