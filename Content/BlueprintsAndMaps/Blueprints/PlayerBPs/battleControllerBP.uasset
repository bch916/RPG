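; Player controller for turn-based battles that turns mouse swipes into the player's skill choice: defend, basic attack, recharge or special attack.
; Left-button press and release positions are compared against a threshold, accepting only single-axis swipes during the player's turn.
; An accepted swipe opens a Tick gate that checks skill energy, updates BattleUI, sets the battle pawn's animation flag and generally ends the turn.
; A successful recharge also updates player health and stats.
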(event `self.ReceiveBeginPlay`
  ;[1 1 1] On Battle Controller Begin Play Show Mouse Cursor
  (set `self.bShowMouseCursor` true)
  (bind _asmain_game_instance (cast `/Game/BlueprintsAndMaps/Blueprints/GameBPs/mainGameInstance` (`GameplayStatics.GetGameInstance`)))
  (set `self.REFMainGameInstance` _asmain_game_instance)
  (bind _foundwidgets (`WidgetBlueprintLibrary.GetAllWidgetsOfClass` "/Game/BlueprintsAndMaps/Blueprints/UI_BPs/BattleUI.BattleUI_C"))
  (set `self.myBattleUI` (`|GetArrayItem` _foundwidgets)))

(event `self.ReceiveTick`
  (params (DeltaSeconds :type "Float (single-precision)"))
  (bind _maingameinstanceplayerobjectbp (`/Game/BlueprintsAndMaps/Blueprints/GameBPs/mainGameInstance.MainGameInstancePlayerObjectBP` (`self.REFMainGameInstance`)))
  (bind _maingameinstanceplayerobjectbp_2 (`/Game/BlueprintsAndMaps/Blueprints/GameBPs/mainGameInstance.MainGameInstancePlayerObjectBP` (`self.REFMainGameInstance`)))
  (bind _maingameinstanceplayerobjectbp_3 (`/Game/BlueprintsAndMaps/Blueprints/GameBPs/mainGameInstance.MainGameInstancePlayerObjectBP` (`self.REFMainGameInstance`)))
  (bind _maingameinstanceplayerobjectbp_4 (`/Game/BlueprintsAndMaps/Blueprints/GameBPs/mainGameInstance.MainGameInstancePlayerObjectBP` (`self.REFMainGameInstance`)))
  (bind _maingameinstanceplayerobjectbp_5 (`/Game/BlueprintsAndMaps/Blueprints/GameBPs/mainGameInstance.MainGameInstancePlayerObjectBP` (`self.REFMainGameInstance`)))
  ;[1 1 1] Enter Gate on Event Tick and Open it When  an Input is registered from Left Mosue Button Event.
  (`/Engine/EditorBlueprintResources/StandardMacros.Gate` true :!label _label
    (:`Exit`
      (if (`self.isSwipeLeft`)
        (bind _returnedskilloftype (`/Game/BlueprintsAndMaps/Blueprints/PlayerBPs/playerObjectBP.returnSkillByType` _maingameinstanceplayerobjectbp "NewEnumerator3"))
        ;[1 1 1] Depending on the Input that was registered and ccording flag set, set the appropriate flag for the Anim BP to carry out an Animation and from there reset this flag.
        (bind _canuseskill (`/Game/BlueprintsAndMaps/Blueprints/PlayerBPs/playerObjectBP.checkPlayerEnergyBeforeSkill` _maingameinstanceplayerobjectbp _returnedskilloftype))
        (`/Game/BlueprintsAndMaps/Blueprints/UI_BPs/BattleUI.playNotEnoughEnergy` (`self.myBattleUI`) _canuseskill)
        (set `/Game/BlueprintsAndMaps/Blueprints/PlayerBPs/battlePlayerBP.isDefending` _canuseskill (cast `/Game/BlueprintsAndMaps/Blueprints/PlayerBPs/battlePlayerBP` (`GameplayStatics.GetPlayerCharacter` 0) :!pure true))
        (elif (`self.isSwipeRight`)
          (bind _returnedskilloftype_2 (`/Game/BlueprintsAndMaps/Blueprints/PlayerBPs/playerObjectBP.returnSkillByType` _maingameinstanceplayerobjectbp_2 "NewEnumerator0"))
          (bind _canuseskill_2 (`/Game/BlueprintsAndMaps/Blueprints/PlayerBPs/playerObjectBP.checkPlayerEnergyBeforeSkill` _maingameinstanceplayerobjectbp_2 _returnedskilloftype_2))
          (`/Game/BlueprintsAndMaps/Blueprints/UI_BPs/BattleUI.playNotEnoughEnergy` (`self.myBattleUI`) _canuseskill_2)
          (set `/Game/BlueprintsAndMaps/Blueprints/PlayerBPs/battlePlayerBP.isBasicAttacking` _canuseskill_2 (cast `/Game/BlueprintsAndMaps/Blueprints/PlayerBPs/battlePlayerBP` (`GameplayStatics.GetPlayerCharacter` 0) :!pure true))
          (elif (`self.isSwipeDown`)
            (bind _returnedskilloftype_3 (`/Game/BlueprintsAndMaps/Blueprints/PlayerBPs/playerObjectBP.returnSkillByType` _maingameinstanceplayerobjectbp_3 "NewEnumerator2"))
            (bind _canuseskill_3 (`/Game/BlueprintsAndMaps/Blueprints/PlayerBPs/playerObjectBP.checkPlayerEnergyBeforeSkill` _maingameinstanceplayerobjectbp_3 _returnedskilloftype_3))
            (`/Game/BlueprintsAndMaps/Blueprints/UI_BPs/BattleUI.playNotEnoughEnergy` (`self.myBattleUI`) _canuseskill_3)
            (bind _output_get (set `/Game/BlueprintsAndMaps/Blueprints/PlayerBPs/battlePlayerBP.isRecharging` _canuseskill_3 (cast `/Game/BlueprintsAndMaps/Blueprints/PlayerBPs/battlePlayerBP` (`GameplayStatics.GetPlayerCharacter` 0) :!pure true)))
            (if _output_get
              (`/Game/BlueprintsAndMaps/Blueprints/PlayerBPs/playerObjectBP.updatePlayerHealthFromRecharge` _maingameinstanceplayerobjectbp_4)
              (`/Game/BlueprintsAndMaps/Blueprints/PlayerBPs/playerObjectBP.updatePlayerStatsStructureFromREF` _maingameinstanceplayerobjectbp_4)
              (else
                (goto _label :!via `Close`)))
            (elif (`self.isSwipeUp`)
              (bind _returnedskilloftype_4 (`/Game/BlueprintsAndMaps/Blueprints/PlayerBPs/playerObjectBP.returnSkillByType` _maingameinstanceplayerobjectbp_5 "NewEnumerator1"))
              (bind _canuseskill_4 (`/Game/BlueprintsAndMaps/Blueprints/PlayerBPs/playerObjectBP.checkPlayerEnergyBeforeSkill` _maingameinstanceplayerobjectbp_5 _returnedskilloftype_4))
              (`/Game/BlueprintsAndMaps/Blueprints/UI_BPs/BattleUI.playNotEnoughEnergy` (`self.myBattleUI`) _canuseskill_4)
              (set `/Game/BlueprintsAndMaps/Blueprints/PlayerBPs/battlePlayerBP.isSpecialAttacking` _canuseskill_4 (cast `/Game/BlueprintsAndMaps/Blueprints/PlayerBPs/battlePlayerBP` (`GameplayStatics.GetPlayerCharacter` 0) :!pure true))
              (else
                (goto _label :!via `Close`))))))
      (set `self.playerTurn` false)
      (goto _label :!via `Close`))))

(event `InputRegistered`
  ;[1 1 1] Enter Gate on Event Tick and Open it When  an Input is registered from Left Mosue Button Event.
  (if (`self.playerTurn`)
    (goto _label :!via `Open`)))

(event `Key|LeftMouseButton`
  (params (Key :type "Key Structure"))
  (bind (_locationx _locationy) (`self.GetMousePosition`))
  (bind (_locationx_2 _locationy_2) (`self.GetMousePosition`))
  (bind _returnvalue (- (`self.releasedX`) (`self.clickedX`)))
  (bind _returnvalue_2 (- (`self.releasedY`) (`self.clickedY`)))
  ;[1 1 1] On Mouse Press, ensure it is Players Turn
  (:`Pressed`
    (if (`self.playerTurn`)
      ;[1 1 1] Reset all Swipe flags
      (set `self.noSwipe` false)
      (set `self.isSwipeUp` false)
      (set `self.isSwipeRight` false)
      (set `self.isSwipeDown` false)
      ;[1 1 1] Get Screen Pos. of Mouse click on Press
      (set `self.isSwipeLeft` false)
      (set `self.clickedX` _locationx_2)
      (set `self.clickedY` _locationy_2)))
  (:`Released`
    (if (`self.playerTurn`)
      ;[1 1 1] On Mouse release, check Delta of Mouse position and see if Swipe was registered.  If so set its Flag and call Input Registered.
      (set `self.releasedX` _locationx)
      (set `self.releasedY` _locationy)
      (if (< _returnvalue_2 0.0)
        (set `self.deltaY` (* _returnvalue_2 -1.0))
        (set `self.isSwipeUp` true)
        (else
          (set `self.deltaY` _returnvalue_2)
          (set `self.isSwipeDown` true)))
      (if (< _returnvalue 0.0)
        (set `self.deltaX` (* _returnvalue -1.0))
        (set `self.isSwipeLeft` true)
        (else
          (set `self.deltaX` _returnvalue)
          (set `self.isSwipeRight` true)))
      (if (<= (`self.deltaX`) (`self.valueLimit`))
        (if (<= (`self.deltaY`) (`self.valueLimit`))
          (set `self.noSwipe` true)
          (else
            (if (`self.isSwipeDown`)
              _
              (else
                _))
            (set `self.isSwipeRight` false)
            (set `self.isSwipeLeft` false)
            (`self.InputRegistered` :!label _label_2)))
        (elif (<= (`self.deltaY`) (`self.valueLimit`))
          (if (`self.isSwipeLeft`)
            _
            (else
              _))
          (set `self.isSwipeDown` false)
          (set `self.isSwipeUp` false)
          (goto _label_2))))))

(fn `UserConstructionScript`)