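; Enemy pawn for both overworld and turn-based battle, handling stats, damage, turn state and stopping non-engaging players on overlap.
; On BeginPlay it builds an EnemyObject from a data table row, restoring current health from the game instance during battle.
; Damage updates the current game mode's UI, then either syncs stats back or shows the end-battle screen.
; Skill damage rolls within percentage bounds of a level-and-power formula; turns use timed delays.
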(event `self.ReceiveBeginPlay`
  ;[1 1 1] On Begin Play Attach Face Decal Mesh to Enemy Pawn
  (`SceneComponent.K2_AttachToComponent` (`self.FaceMesh`) (`self.enemyMesh`) "FaceSocket" "SnapToTarget" "SnapToTarget" "SnapToTarget" true)
  (set `self.isIdle` true)
  (bind _asmain_game_instance (cast `/Game/BlueprintsAndMaps/Blueprints/GameBPs/mainGameInstance` (`GameplayStatics.GetGameInstance`)))
  (set `self.REFMainGameInstance` _asmain_game_instance)
  (`self.setEnemyStats`))

(event `enemyTargeted`
  ;[1 1 1] Interaction from Player Controller can call this event to set Enemy into Reacting State
  (set `self.isReacting` true))

(event `self.ReceiveActorBeginOverlap`
  (params (OtherActor :type "Actor Object Reference"))
  ;[1 0.8061 0] Prevents Players from walking through Enemies. Upon something Overlapping this Enemy pawn, check to see if thats a Player Pawn and see if it is NOT Engaging, if so Stop Its movement(this may be redundant), else ignore.
  (bind _asoverworld_player_bp (cast `/Game/BlueprintsAndMaps/Blueprints/PlayerBPs/overworldPlayerBP` OtherActor))
  (if (not (`/Game/BlueprintsAndMaps/Blueprints/PlayerBPs/overworldPlayerBP.isEngaging` _asoverworld_player_bp))
    (`MovementComponent.StopMovementImmediately` (`Character.CharacterMovement` (`GameplayStatics.GetPlayerCharacter` 0)))))

(event `takeDamage`
  (params (damageNumber :type Integer))
  (bind _returnvalue (`GameplayStatics.GetGameMode`))
  (bind _returnvalue_2 (`GameplayStatics.GetGameMode`))
  ;[1 1 1] Enemy Takes Damage.  Subtract incoming damage from health and pass the damage number to the Game Modes Current UI to display dmg.
  (set `self.REFCurrentHealth` (- (`self.REFCurrentHealth`) (`KismetMathLibrary.Conv_IntToDouble` damageNumber)))
  (bind _asmain_game_mode (cast `/Game/BlueprintsAndMaps/Blueprints/GameBPs/mainGameMode` _returnvalue)
    (:`then`
      (bind _currentoverworldui (`/Game/BlueprintsAndMaps/Blueprints/GameBPs/mainGameMode.currentOverworldUI` _asmain_game_mode))
      (set `/Game/BlueprintsAndMaps/Blueprints/UI_BPs/OverworldUI.enemyDamagedNumber` damageNumber _currentoverworldui)
      (if (`self.isDefeated`)
        ;[1 1 1] Check if Damage is defating the Enemy and if so set Flag fo Defeated and call Change Mob Spawn Count on Game Instance. Delay 1 second and DEstroy the Enemy Pawn.
        (bind _asbattle_game_mode (cast `/Game/BlueprintsAndMaps/Blueprints/GameBPs/battleGameMode` _returnvalue_2 :!label _label)
          (:`then`
            (`/Game/BlueprintsAndMaps/Blueprints/GameBPs/battleGameMode.displayEndBattleScreen` _asbattle_game_mode))
          (:`CastFailed`
            (bind _asmain_game_mode_2 (cast `/Game/BlueprintsAndMaps/Blueprints/GameBPs/mainGameMode` _returnvalue_2))
            (`/Game/BlueprintsAndMaps/Blueprints/GameBPs/mainGameMode.displayEndBattleScreen` _asmain_game_mode_2)))
        (else
          (`/Game/BlueprintsAndMaps/Blueprints/UI_BPs/OverworldUI.enemyTakesDamage` _currentoverworldui damageNumber)
          (if (<= (`self.REFCurrentHealth`) 0.0) :!label _label_2
            (set `self.isDefeated` true)
            (goto _label)
            (else
              (set `/Game/BlueprintsAndMaps/Blueprints/GameBPs/mainGameInstance.currentEnemyHealth` (`self.REFCurrentHealth`) (cast `/Game/BlueprintsAndMaps/Blueprints/GameBPs/mainGameInstance` (`GameplayStatics.GetGameInstance`) :!pure true))
              (`self.updateEnemyStatsFromREF`))))))
    (:`CastFailed`
      (bind _asbattle_game_mode_2 (cast `/Game/BlueprintsAndMaps/Blueprints/GameBPs/battleGameMode` _returnvalue))
      (bind _currentbattleuiinstance (`/Game/BlueprintsAndMaps/Blueprints/GameBPs/battleGameMode.currentBattleUIInstance` _asbattle_game_mode_2))
      (bind _output_get (set `/Game/BlueprintsAndMaps/Blueprints/UI_BPs/BattleUI.enemyDamagedNumber` damageNumber _currentbattleuiinstance))
      (if (not (`self.isDefeated`))
        (`/Game/BlueprintsAndMaps/Blueprints/UI_BPs/BattleUI.enemyTakesDamage` _currentbattleuiinstance _output_get)
        (goto _label_2)))))

(event `updateEnemyPower`
  (`self.setEnemyPower`))

(event `setEnemyToBattleState`
  (bind _refmaingameinstance (`self.REFMainGameInstance`))
  ;[1 0.7963 0] Comment
  (set `/Game/BlueprintsAndMaps/Blueprints/GameBPs/mainGameInstance.currentBattleEnemyOverworldData` self _refmaingameinstance)
  (set `self.enemyObject` (`/Game/BlueprintsAndMaps/Blueprints/GameBPs/mainGameInstance.currentBattleEnemyObject` _refmaingameinstance))
  (`ActorComponent.Deactivate` (`self.OverLapSphere`))
  (`self.K2_SetActorRotation` (struct :`Yaw` -90.0)))

(event `setEnemyToOverWorldState`
  ;[1 0.7963 0] Comment
  (`self.updateEnemyREFFromStats`))

(event `takeTurn`
  ;[1 1 1] Transferred the Take Turn Event from the old Battle Enemy BP.
  (set `self.isEnemyTurn` true)
  (`KismetSystemLibrary.Delay` (`self.enemyThinkTime`))
  (set `self.isAttacking` true))

(event `finishTurn`
  (bind _asbattle_game_mode (cast `/Game/BlueprintsAndMaps/Blueprints/GameBPs/battleGameMode` (`GameplayStatics.GetGameMode`) :!pure true))
  (set `self.isEnemyTurn` false)
  (`KismetSystemLibrary.Delay` (`/Game/BlueprintsAndMaps/Blueprints/GameBPs/battleGameMode.turnDelay` _asbattle_game_mode))
  (`/Game/BlueprintsAndMaps/Blueprints/GameBPs/battleGameMode.enemyFinishedTurn` _asbattle_game_mode))

(event `updateEnemyREFFromStats`
  (bind (_currenthealth _maxhealth _currentlevel _basepower) (break `/Game/BlueprintsAndMaps/Blueprints/EnemyBPs/EnemyStatsStructure` (`.enemyStatsStructure_24_4EE90FF34717CAB233423F81FF46FAA0` (break `/Game/BlueprintsAndMaps/Blueprints/EnemyBPs/EnemyDataStructure` (`/Game/BlueprintsAndMaps/Blueprints/EnemyBPs/enemyObject_BP.enemyDataStructure` (`self.enemyObject`))))))
  ;[1 1 1] SImilar concept on Player Object...but the Enemy Pawn handles its own object as I am okay with it being destroyed and re created at this point.
  (set `self.REFCurrentHealth` (`KismetMathLibrary.Conv_IntToDouble` _currenthealth))
  (set `self.REFMaxHealth` (`KismetMathLibrary.Conv_IntToDouble` _maxhealth))
  (set `self.REFEnemyLevel` _currentlevel)
  (set `self.REFBasePower` _basepower))

(event `updateEnemyStatsFromREF`
  (bind (_enemydatastructure_enemyname _enemydatastructure_enemyid _enemydatastructure_enemymodel _enemydatastructure_enemyclass _enemydatastructure_enemyanimbp _enemydatastructure_enemylootstructure _enemydatastructure_enemystatsstructure _enemydatastructure_enemyskillarray) (break `/Game/BlueprintsAndMaps/Blueprints/EnemyBPs/EnemyDataStructure` (`/Game/BlueprintsAndMaps/Blueprints/EnemyBPs/enemyObject_BP.enemyDataStructure` (`self.enemyObject`))))
  ;[1 1 1] SImilar concept on Player Object...but the Enemy Pawn handles its own object as I am okay with it being destroyed and re created at this point.
  (bind _output_get (set `/Game/BlueprintsAndMaps/Blueprints/EnemyBPs/enemyObject_BP.enemyDataStructure` (make `/Game/BlueprintsAndMaps/Blueprints/EnemyBPs/EnemyDataStructure` _enemydatastructure_enemyname _enemydatastructure_enemyid _enemydatastructure_enemymodel _enemydatastructure_enemyclass _enemydatastructure_enemyanimbp _enemydatastructure_enemylootstructure (make `/Game/BlueprintsAndMaps/Blueprints/EnemyBPs/EnemyStatsStructure` (`KismetMathLibrary.FTrunc` (`self.REFCurrentHealth`)) (`KismetMathLibrary.FTrunc` (`self.REFMaxHealth`)) (`self.REFEnemyLevel`) (`self.REFBasePower`)) _enemydatastructure_enemyskillarray) (`self.enemyObject`)))
  (set `/Game/BlueprintsAndMaps/Blueprints/EnemyBPs/enemyObject_BP.enemyDataStructure` _output_get (`/Game/BlueprintsAndMaps/Blueprints/GameBPs/mainGameInstance.currentBattleEnemyObject` (`self.REFMainGameInstance`))))

(fn `calcDamageBySkillIndex`
  (params (skillIndex :type Integer))
  (returns (damageBySkill :type Integer))
  (bind (_mindamagepercent _maxdamagepercent) (break `/Game/BlueprintsAndMaps/Blueprints/WeaponAndSkillsBPs/SkillStatsStructure` (`.SkillStatsStructure_32_E2D795DC4E3A7DC2AF5A5BAE0D6F8560` (break `/Game/BlueprintsAndMaps/Blueprints/WeaponAndSkillsBPs/SkillDataStructure` (`|GetArrayItem` (`.enemySkillArray_22_E505B6554D75399C268272B68FD36472` (break `/Game/BlueprintsAndMaps/Blueprints/EnemyBPs/EnemyDataStructure` (`/Game/BlueprintsAndMaps/Blueprints/EnemyBPs/enemyObject_BP.enemyDataStructure` (`self.enemyObject`)))) skillIndex)))))
  (bind _power (`self.calcTotalPower`))
  (return (`KismetMathLibrary.RandomIntegerInRange` (`KismetMathLibrary.FTrunc` (* _power _mindamagepercent)) (`KismetMathLibrary.FTrunc` (* _power _maxdamagepercent)))))

(fn `calcTotalPower`
  (returns (Power :type Integer))
  (return (`KismetMathLibrary.FTrunc` (* (`KismetMathLibrary.Log` (* (`KismetMathLibrary.Conv_IntToDouble` (+ (`self.REFEnemyLevel`) 1)) (`self.unitPowerLvlModifier`)) 2.0) (+ (`KismetMathLibrary.MultiplyMultiply_FloatFloat` (`KismetMathLibrary.Conv_IntToDouble` (* (`self.REFBasePower`) (`self.REFEnemyLevel`))) 2.0) (`KismetMathLibrary.Conv_IntToDouble` (+ (`self.REFBasePower`) (`KismetMathLibrary.FTrunc` (* (`self.REFBasePower`) (`self.unitPowerLvlModifier`))))))))))

(fn `setEnemyPower`
  (bind (_enemydatastructure_enemyname _enemydatastructure_enemyid _enemydatastructure_enemymodel _enemydatastructure_enemyclass _enemydatastructure_enemyanimbp _enemydatastructure_enemylootstructure _enemydatastructure_enemystatsstructure) (break `/Game/BlueprintsAndMaps/Blueprints/EnemyBPs/EnemyDataStructure` (`/Game/BlueprintsAndMaps/Blueprints/EnemyBPs/enemyObject_BP.enemyDataStructure` (`self.enemyObject`))))
  (set `self.REFBasePower` (`.basePower_10_E8DAFC6A40C68ED0525920BE2DAEBAE4` (break `/Game/BlueprintsAndMaps/Blueprints/EnemyBPs/EnemyStatsStructure` _enemydatastructure_enemystatsstructure))))

(fn `setEnemyStats`
  (bind _returnvalue (`|GetDataTableRow` "/Game/BlueprintsAndMaps/Blueprints/EnemyBPs/EnemyDataTable.EnemyDataTable" (`self.enemyName`))
    (:`then`
      (bind _returnvalue_2 (`|GenericCreateObject` "/Game/BlueprintsAndMaps/Blueprints/EnemyBPs/enemyObject_BP.enemyObject_BP_C" self))
      (bind _output_get (set `self.enemyObject` _returnvalue_2))
      (if (`/Game/BlueprintsAndMaps/Blueprints/GameBPs/mainGameInstance.isBattle?` (`self.REFMainGameInstance`))
        (bind (_enemyname _enemyid _enemymodel _enemyclass _enemyanimbp _enemylootstructure _enemystatsstructure _enemyskillarray) (break `/Game/BlueprintsAndMaps/Blueprints/EnemyBPs/EnemyDataStructure` _returnvalue))
        (set `/Game/BlueprintsAndMaps/Blueprints/EnemyBPs/enemyObject_BP.enemyDataStructure` (make `/Game/BlueprintsAndMaps/Blueprints/EnemyBPs/EnemyDataStructure` _enemyname _enemyid _enemymodel _enemyclass _enemyanimbp _enemylootstructure (make `/Game/BlueprintsAndMaps/Blueprints/EnemyBPs/EnemyStatsStructure` (`KismetMathLibrary.FTrunc` (`/Game/BlueprintsAndMaps/Blueprints/GameBPs/mainGameInstance.currentEnemyHealth` (`self.REFMainGameInstance`))) (`.maxHealth_4_868A89B94C3B16FB4FEF4AB6B6BFA5EF` (break `/Game/BlueprintsAndMaps/Blueprints/EnemyBPs/EnemyStatsStructure` _enemystatsstructure)) (`.currentLevel_17_397BF91543B198A136CF18B3B399FC1A` (break `/Game/BlueprintsAndMaps/Blueprints/EnemyBPs/EnemyStatsStructure` _enemystatsstructure)) (`.basePower_10_E8DAFC6A40C68ED0525920BE2DAEBAE4` (break `/Game/BlueprintsAndMaps/Blueprints/EnemyBPs/EnemyStatsStructure` _enemystatsstructure))) _enemyskillarray) (`self.enemyObject`))
        (`self.updateEnemyREFFromStats`)
        (else
          (bind (_enemyname_2 _enemyid_2 _enemymodel_2 _enemyclass_2 _enemyanimbp_2 _enemylootstructure_2 _enemystatsstructure_2 _enemyskillarray_2) (break `/Game/BlueprintsAndMaps/Blueprints/EnemyBPs/EnemyDataStructure` _returnvalue))
          (set `/Game/BlueprintsAndMaps/Blueprints/EnemyBPs/enemyObject_BP.enemyDataStructure` (make `/Game/BlueprintsAndMaps/Blueprints/EnemyBPs/EnemyDataStructure` _enemyname_2 _enemyid_2 _enemymodel_2 _enemyclass_2 _enemyanimbp_2 _enemylootstructure_2 (make `/Game/BlueprintsAndMaps/Blueprints/EnemyBPs/EnemyStatsStructure` (break `/Game/BlueprintsAndMaps/Blueprints/EnemyBPs/EnemyStatsStructure` _enemystatsstructure_2) (`.maxHealth_4_868A89B94C3B16FB4FEF4AB6B6BFA5EF` (break `/Game/BlueprintsAndMaps/Blueprints/EnemyBPs/EnemyStatsStructure` _enemystatsstructure_2)) (`.currentLevel_17_397BF91543B198A136CF18B3B399FC1A` (break `/Game/BlueprintsAndMaps/Blueprints/EnemyBPs/EnemyStatsStructure` _enemystatsstructure_2)) (`.basePower_10_E8DAFC6A40C68ED0525920BE2DAEBAE4` (break `/Game/BlueprintsAndMaps/Blueprints/EnemyBPs/EnemyStatsStructure` _enemystatsstructure_2))) _enemyskillarray_2) _output_get)
          (`self.updateEnemyREFFromStats`))))))

(fn `UserConstructionScript`)